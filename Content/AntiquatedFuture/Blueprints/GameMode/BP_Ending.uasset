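; BP_Ending is a trigger actor that ends the game when the robot character enters its box.
; On overlap the character speaks a line, then after a delay loses input while the first-person game mode removes the quest.
; A WBP_FadeScreen widget then plays its fade-out animation, and the L_EndScreen level opens shortly after.
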(event OnComponentBeginOverlap(Box)
  (params (OverlappedComponent :type Primitive%20Component%20Object%20Reference) (OtherActor :type Actor%20Object%20Reference) (OtherComp :type Primitive%20Component%20Object%20Reference) (OtherBodyIndex :type Integer) (bFromSweep :type Boolean) (SweepResult :type Hit%20Result%20Structure%20%28by%20ref%29))
  (bind _asbp_robot_character (Utilities|Casting|CastToBP_RobotCharacter OtherActor))
  (Variables|/Game/AntiquatedFuture/Blueprints/BP_RobotCharacter.BP_RobotCharacter_C|SetSpeechText _asbp_robot_character "I am robot.")
  (Default|Speech _asbp_robot_character)
  (Utilities|FlowControl|Delay 5.0)
  (Input|DisableInput _asbp_robot_character (Game|GetPlayerController 0))
  (bind _asbp_gamemode_first_person (Utilities|Casting|CastToBP_GamemodeFirstPerson (Game|GetGameMode)))
  (Default|RemoveQuest _asbp_gamemode_first_person)
  (bind _returnvalue (UserInterface|CreateWidget "/Game/AntiquatedFuture/UI/WBP_FadeScreen.WBP_FadeScreen_C"))
  (UserInterface|Viewport|AddtoViewport _returnvalue 0)
  (UserInterface|Animation|PlayAnimation _returnvalue (Variables|/Game/AntiquatedFuture/UI/WBP_FadeScreen.WBP_FadeScreen_C|GetFadeOut _returnvalue) 0.0 1 "Forward" 1.0 false)
  (Utilities|FlowControl|Delay 1.0)
  (Game|OpenLevel(byName) "L_EndScreen"))

(event EventBeginPlay)

(event Collision|EventActorBeginOverlap
  (params (OtherActor :type Actor%20Object%20Reference)))

(event EventTick
  (params (DeltaSeconds :type Float%20%28single-precision%29)))

(fn ConstructionScript)