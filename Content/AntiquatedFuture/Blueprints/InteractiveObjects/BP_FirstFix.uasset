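; BP_FirstFix is a one-time interactable that upgrades the robot player's view by swapping its camera effect, likely the first repair in the game.
; On interaction it removes its pipe mesh, disables player input and plays a rustle sound with a screen fade.
; Between two timed fade widgets, it replaces the first camera modifier with the black-and-white one through PCM_CameraManager.
; It then restores input and destroys itself.
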(event Custom|ChangeModifier
  (bind _aspcm_camera_manager (Utilities|Casting|CastToPCM_CameraManager (Game|GetPlayerCameraManager 0)))
  (bind _returnvalue (Game|Player|FindCameraModifierbyClass _aspcm_camera_manager "/Game/AntiquatedFuture/Blueprints/CameraModifier/CM_1CameraModifier.CM_1CameraModifier_C"))
  (Game|Player|RemoveCameraModifier _aspcm_camera_manager _returnvalue)
  (Game|Player|AddNewCameraModifier _aspcm_camera_manager "/Game/AntiquatedFuture/Blueprints/CameraModifier/CM_2CameraModifier_blackwhite.CM_2CameraModifier_blackwhite_C"))

(event EventBeginPlay
  (bind _asbp_robot_character (Utilities|Casting|CastToBP_RobotCharacter (Game|GetPlayerCharacter 0)))
  (Variables|Default|SetAs%20BP%20Robot%20Character _asbp_robot_character))

(event EventInteractive
  (bind _returnvalue (Game|GetPlayerController 0))
  (Utilities|FlowControl|DoOnce false
    (:Completed
      (Components|DestroyComponent (Variables|Default|GetSM_Slums_Pipe_02a))
      (Input|DisableInput (Variables|Default|GetAs%20BP%20Robot%20Character) _returnvalue)
      (bind _returnvalue_2 (UserInterface|CreateWidget "/Game/AntiquatedFuture/UI/WBP_FadeScreen.WBP_FadeScreen_C" _returnvalue))
      (UserInterface|Viewport|AddtoViewport _returnvalue_2 0)
      (Audio|PlaySound2D "/Game/AntiquatedFuture/Sounds/RoboSounds/science-fiction-robot-rustle-click-04_Cue.science-fiction-robot-rustle-click-04_Cue" 1.0 1.0 0.0 0 0)
      (UserInterface|Animation|PlayAnimation _returnvalue_2 (Variables|/Game/AntiquatedFuture/UI/WBP_FadeScreen.WBP_FadeScreen_C|GetFadeOut _returnvalue_2) 0.0 1 "Forward" 1.0 false)
      (Utilities|FlowControl|Delay 1.0)
      (CallFunction|ChangeModifier)
      (Widget|RemovefromParent _returnvalue_2)
      (bind _returnvalue_3 (UserInterface|CreateWidget "/Game/AntiquatedFuture/UI/WBP_FadeScreen.WBP_FadeScreen_C" (Game|GetPlayerController 0)))
      (UserInterface|Viewport|AddtoViewport _returnvalue_3 0)
      (UserInterface|Animation|PlayAnimation _returnvalue_3 (Variables|/Game/AntiquatedFuture/UI/WBP_FadeScreen.WBP_FadeScreen_C|GetFadeOut _returnvalue_3) 0.0 1 "Forward" 1.0 false)
      (Utilities|FlowControl|Delay 1.0)
      (Widget|RemovefromParent _returnvalue_3)
      (Input|EnableInput (Variables|Default|GetAs%20BP%20Robot%20Character) (Game|GetPlayerController 0))
      (Actor|DestroyActor))))

(fn ConstructionScript)