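; Interactive pickup for the Bargaining stage, a slums pipe mesh with a point light that advances the game when used.
; BeginPlay caches the robot player character and the first-person game mode.
; The first interaction removes the mesh and light, plays a robot click sound and swaps the red camera modifier for the yellow one.
; It then calls Bargaining on the game mode and destroys itself.
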(event Custom|ChangeModifier
  (bind _aspcm_camera_manager (Utilities|Casting|CastToPCM_CameraManager (Game|GetPlayerCameraManager 0)))
  (bind _returnvalue (Game|Player|FindCameraModifierbyClass _aspcm_camera_manager "/Game/AntiquatedFuture/Blueprints/CameraModifier/CM_3CameraModifier_red.CM_3CameraModifier_red_C"))
  (Game|Player|RemoveCameraModifier _aspcm_camera_manager _returnvalue)
  (Game|Player|AddNewCameraModifier _aspcm_camera_manager "/Game/AntiquatedFuture/Blueprints/CameraModifier/CM_4CameraModifier_yellow.CM_4CameraModifier_yellow_C"))

(event Custom|NewStage
  (Default|Bargaining (Variables|Default|GetAs%20BP%20Gamemode%20First%20Person)))

(event EventBeginPlay
  (bind _asbp_robot_character (Utilities|Casting|CastToBP_RobotCharacter (Game|GetPlayerCharacter 0)))
  (Variables|Default|SetAs%20BP%20Robot%20Character _asbp_robot_character)
  (bind _asbp_gamemode_first_person (Utilities|Casting|CastToBP_GamemodeFirstPerson (Game|GetGameMode)))
  (Variables|Default|SetAs%20BP%20Gamemode%20First%20Person _asbp_gamemode_first_person))

(event EventInteractive
  (Utilities|FlowControl|DoOnce false
    (:Completed
      (Components|DestroyComponent (Variables|Default|GetSM_Slums_Pipe_02a))
      (Audio|PlaySound2D "/Game/AntiquatedFuture/Sounds/RoboSounds/science-fiction-robot-rustle-click-04_Cue.science-fiction-robot-rustle-click-04_Cue" 1.0 1.0 0.0 0 0)
      (CallFunction|ChangeModifier)
      (CallFunction|NewStage)
      (Actor|DestroyActor))))

(fn ConstructionScript)