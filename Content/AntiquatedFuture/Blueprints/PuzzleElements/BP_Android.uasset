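; BP_Android is a quest-giver NPC that opens a bridge once the player has found its amplifier module.
; On interaction it checks the gamemode's AndroidItemRecieved flag and sends a dialogue line to the robot player character's Speech function.
; The first interaction with the item completes the quest and makes the BP_Bridge mesh visible and collidable.
; DoOnce gates with five-second resets throttle the repeatable hint and post-quest lines.
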(event Custom|PlatformAppears
  (bind _returnvalue (Actor|GetActorOfClass "/Game/AntiquatedFuture/Blueprints/PuzzleElements/BP_Bridge.BP_Bridge_C"))
  (Rendering|SetVisibility (Variables|/Game/AntiquatedFuture/Blueprints/PuzzleElements/BP_Bridge.BP_Bridge_C|GetBridge _returnvalue) true false)
  (Collision|SetCollisionEnabled (Variables|/Game/AntiquatedFuture/Blueprints/PuzzleElements/BP_Bridge.BP_Bridge_C|GetBridge _returnvalue) "QueryAndPhysics"))

(event EventInteractive
  (bind _as_bp_robot_character (Variables|Default|GetAs%20BP%20Robot%20Character))
  (bind _as_bp_robot_character_2 (Variables|Default|GetAs%20BP%20Robot%20Character))
  (if (not (Variables|/Game/AntiquatedFuture/Blueprints/GameMode/BP_GamemodeFirstPerson.BP_GamemodeFirstPerson_C|GetAndroidItemRecieved (Variables|Default|GetAs%20BP%20Gamemode%20First%20Person)))
    (Utilities|FlowControl|DoOnce false :!label _label
      (:Completed
        (Variables|/Game/AntiquatedFuture/Blueprints/BP_RobotCharacter.BP_RobotCharacter_C|SetSpeechText _as_bp_robot_character_2 "Android: Locate the amplifier module, and I'll assist you further.")
        (Default|Speech _as_bp_robot_character_2)
        (Utilities|FlowControl|Delay 5.0)
        (goto _label Reset)))
    (elif (not (Variables|Default|GetQuestCompleted))
      (Variables|/Game/AntiquatedFuture/Blueprints/BP_RobotCharacter.BP_RobotCharacter_C|SetSpeechText _as_bp_robot_character "Android: The emptiness in my ears is gone... The path for you is open.")
      (Default|Speech _as_bp_robot_character)
      (CallFunction|PlatformAppears)
      (Variables|Default|SetQuestCompleted true)
      (else
        (Utilities|FlowControl|DoOnce false :!label _label_2
          (:Completed
            (Variables|/Game/AntiquatedFuture/Blueprints/BP_RobotCharacter.BP_RobotCharacter_C|SetSpeechText _as_bp_robot_character "Android: I can now hear the insects scuttling on my body.")
            (Default|Speech _as_bp_robot_character)
            (Utilities|FlowControl|Delay 5.0)
            (goto _label_2 Reset)))))))

(event EventBeginPlay
  (bind _asbp_robot_character (Utilities|Casting|CastToBP_RobotCharacter (Game|GetPlayerCharacter 0)))
  (Variables|Default|SetAs%20BP%20Robot%20Character _asbp_robot_character)
  (bind _asbp_gamemode_first_person (Utilities|Casting|CastToBP_GamemodeFirstPerson (Game|GetGameMode)))
  (Variables|Default|SetAs%20BP%20Gamemode%20First%20Person _asbp_gamemode_first_person))

(fn ConstructionScript)