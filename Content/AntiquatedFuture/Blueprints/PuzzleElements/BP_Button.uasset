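; BP_Button is a puzzle-element pressure button that reacts to BP_RobotCharacter, with no output to other objects.
; Overlapping its SphereCollision plays a metal rattle and a timeline that lowers the Cylinder.
; Ending overlap with the Cylinder, rather than the sphere, prints a debug string and reverses the timeline.
; Each update lerps from the Cylinder's current location toward 10 units below it, so no rest position is stored.
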(event OnComponentBeginOverlap(SphereCollision)
  (params (OverlappedComponent :type Primitive%20Component%20Object%20Reference) (OtherActor :type Actor%20Object%20Reference) (OtherComp :type Primitive%20Component%20Object%20Reference) (OtherBodyIndex :type Integer) (bFromSweep :type Boolean) (SweepResult :type Hit%20Result%20Structure%20%28by%20ref%29))
  (bind _cylinder (Variables|Default|GetCylinder))
  (bind _relativelocation (Variables|/Script/Engine.SceneComponent|GetRelativeLocation _cylinder))
  (Utilities|Casting|CastToBP_RobotCharacter OtherActor)
  (Audio|PlaySoundatLocation "/Game/SoulCity/Sound/Cue/AmbientNonLooping/MetalPanel_ThinRattle_01_Cue.MetalPanel_ThinRattle_01_Cue" (Transformation|GetWorldLocation (Variables|Default|GetCylinder)) "0, 0, 0" 1.0 1.0 0.0 0 0 0 0)
  (bind _alpha (Timeline|Timeline Play)
    (:Update
      (Transformation|SetRelativeLocation _cylinder (Math|Vector|Lerp(Vector) (Variables|/Script/Engine.SceneComponent|GetRelativeLocation _cylinder) (Math|Vector|MakeVector (.x _relativelocation) (.y _relativelocation) (- (.z _relativelocation) 1e+01)) _alpha) false false))))

(event OnComponentEndOverlap(Cylinder)
  (params (OverlappedComponent :type Primitive%20Component%20Object%20Reference) (OtherActor :type Actor%20Object%20Reference) (OtherComp :type Primitive%20Component%20Object%20Reference) (OtherBodyIndex :type Integer))
  (bind _cylinder (Variables|Default|GetCylinder))
  (bind _relativelocation (Variables|/Script/Engine.SceneComponent|GetRelativeLocation _cylinder))
  (Utilities|Casting|CastToBP_RobotCharacter OtherActor)
  (Development|PrintString "Hello")
  (bind _alpha (Timeline|Timeline Reverse)
    (:Update
      (Transformation|SetRelativeLocation _cylinder (Math|Vector|Lerp(Vector) (Variables|/Script/Engine.SceneComponent|GetRelativeLocation _cylinder) (Math|Vector|MakeVector (.x _relativelocation) (.y _relativelocation) (- (.z _relativelocation) 1e+01)) _alpha) false false))))

(event EventBeginPlay)

(event Collision|EventActorBeginOverlap
  (params (OtherActor :type Actor%20Object%20Reference)))

(event EventTick
  (params (DeltaSeconds :type Float%20%28single-precision%29)))

(fn ConstructionScript)