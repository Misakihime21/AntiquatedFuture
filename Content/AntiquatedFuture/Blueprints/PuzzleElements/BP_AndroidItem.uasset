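; BP_AndroidItem is an interactable puzzle pickup that represents an item requested of the player's robot character.
; On BeginPlay it caches the player's BP_RobotCharacter and the BP_GamemodeFirstPerson game mode.
; When interacted with, it removes its light and cube, plays a robot vocal notification, and sets the game mode's AndroidItemRecieved flag.
; It then has the robot announce receipt through its Speech function and destroys itself.
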(event EventInteractive
  (bind _as_bp_robot_character (Variables|Default|GetAs%20BP%20Robot%20Character))
  (Components|DestroyComponent (Variables|Default|GetPointLight))
  (Audio|PlaySound2D "/Game/AntiquatedFuture/Sounds/RoboSounds/ui-notification-robot-vocal-01.ui-notification-robot-vocal-01" 1.0 1.0 0.0 0 0)
  (Variables|/Game/AntiquatedFuture/Blueprints/GameMode/BP_GamemodeFirstPerson.BP_GamemodeFirstPerson_C|SetAndroidItemRecieved (Variables|Default|GetAs%20BP%20Gamemode%20First%20Person) true)
  (Variables|/Game/AntiquatedFuture/Blueprints/BP_RobotCharacter.BP_RobotCharacter_C|SetSpeechText _as_bp_robot_character "The requested item recieved.")
  (Default|Speech _as_bp_robot_character)
  (Actor|DestroyActor))

(event EventBeginPlay
  (bind _asbp_robot_character (Utilities|Casting|CastToBP_RobotCharacter (Game|GetPlayerCharacter 0)))
  (Variables|Default|SetAs%20BP%20Robot%20Character _asbp_robot_character)
  (bind _asbp_gamemode_first_person (Utilities|Casting|CastToBP_GamemodeFirstPerson (Game|GetGameMode)))
  (Variables|Default|SetAs%20BP%20Gamemode%20First%20Person _asbp_gamemode_first_person))

(fn ConstructionScript)