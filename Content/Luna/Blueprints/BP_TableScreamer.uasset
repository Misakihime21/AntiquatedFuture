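; BP_TableScreamer is a one-time jump scare in which a coffee table flies up, falls and breaks when Luna comes near.
; One trigger volume plays a suspense sound on Luna's first overlap.
; A second drives two lerp timelines that move the table to a target position and back, separated by delays.
; It then plays a collapse sound, swaps in the broken mesh and briefly shows a Luna monologue widget.
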(event OnComponentBeginOverlap(CollisionSuspence)
  (params (OverlappedComponent :type Primitive%20Component%20Object%20Reference) (OtherActor :type Actor%20Object%20Reference) (OtherComp :type Primitive%20Component%20Object%20Reference) (OtherBodyIndex :type Integer) (bFromSweep :type Boolean) (SweepResult :type Hit%20Result%20Structure%20%28by%20ref%29))
  (Utilities|Casting|CastToBP_LunaCharacter OtherActor)
  (Utilities|FlowControl|DoOnce false
    (:Completed
      (Audio|PlaySoundatLocation "/Game/Luna/Sounds/mixkit-cinematic-suspense-swell-786.mixkit-cinematic-suspense-swell-786" (Transformation|GetWorldLocation (Variables|Default|GetSurpriseCoffeeTable)) "0, 0, 0" 1.0 1.0 0.0 0 0 0 0))))

(event OnComponentBeginOverlap(CollisionScreamer)
  (params (OverlappedComponent :type Primitive%20Component%20Object%20Reference) (OtherActor :type Actor%20Object%20Reference) (OtherComp :type Primitive%20Component%20Object%20Reference) (OtherBodyIndex :type Integer) (bFromSweep :type Boolean) (SweepResult :type Hit%20Result%20Structure%20%28by%20ref%29))
  (bind _surprisecoffeetable (Variables|Default|GetSurpriseCoffeeTable))
  (Utilities|Casting|CastToBP_LunaCharacter OtherActor)
  (Utilities|FlowControl|DoOnce false
    (:Completed
      (CallFunction|Flying)
      (Utilities|FlowControl|Delay 1.0)
      (CallFunction|Falling)
      (Utilities|FlowControl|Delay 1.0)
      (Audio|PlaySoundatLocation "/Game/StarterContent/Audio/Collapse01.Collapse01" (Transformation|GetWorldLocation _surprisecoffeetable) "0, 0, 0" 1.0 1.0 0.0 0 0 0 0)
      (Components|DestroyComponent _surprisecoffeetable)
      (Rendering|SetVisibility (Variables|Default|GetSurpriseCoffeeTable_Broken) true false)
      (bind _returnvalue (UserInterface|CreateWidget "/Game/Luna/UI/Example_WPB_LunaMonologue.Example_WPB_LunaMonologue_C" (Game|GetPlayerController 0) (Variables|Default|GetLuna%20Says)))
      (UserInterface|Viewport|AddtoViewport _returnvalue 0)
      (Utilities|FlowControl|Delay 1.5)
      (Widget|RemovefromParent _returnvalue))))

(event Custom|Flying
  (bind _surprisecoffeetable (Variables|Default|GetSurpriseCoffeeTable))
  (bind _alpha (Timeline|Timeline Play)
    (:Update
      (Transformation|SetRelativeLocation _surprisecoffeetable (Math|Vector|Lerp(Vector) (Variables|/Script/Engine.SceneComponent|GetRelativeLocation _surprisecoffeetable) (Variables|Default|GetNew%20Position) _alpha) false false))))

(event Custom|Falling
  (bind _surprisecoffeetable (Variables|Default|GetSurpriseCoffeeTable))
  (bind _alpha (Timeline|Timeline_0 Play)
    (:Update
      (Transformation|SetRelativeLocation _surprisecoffeetable (Math|Vector|Lerp(Vector) (Variables|Default|GetNew%20Position) (Variables|/Script/Engine.SceneComponent|GetRelativeLocation _surprisecoffeetable) _alpha) false false))))

(fn ConstructionScript)