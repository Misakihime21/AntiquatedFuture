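; Interactive basement door that checks the first-person game mode's SearchMode and HasKey flags before it opens.
; With both set, the lock barricade is destroyed once with a key sound, and a FlipFlop timeline swings the door open or closed with a creak.
; Otherwise it plays a locked sound and shows a three-second item or Luna monologue widget, guarded against repeat triggers.
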(event Custom|LockOpens
  (Utilities|FlowControl|DoOnce false
    (:Completed
      (Audio|PlaySoundatLocation "/Game/Luna/Sounds/mixkit-dropping-keys-in-the-floor-2839.mixkit-dropping-keys-in-the-floor-2839" (Transformation|GetWorldLocation (Variables|Default|GetDoorBarricade_a)) "0, 0, 0" 1.0 1.0 0.0 0 0 0 0)
      (Components|DestroyComponent (Variables|Default|GetDoorBarricade_a)))))

(event EventBeginPlay
  (bind _asbp_lgamemode_first_person (Utilities|Casting|CastToExample_BP_LGamemodeFirstPerson (Game|GetGameMode)))
  (Variables|Default|SetAs%20BP%20LGamemode%20First%20Person _asbp_lgamemode_first_person))

(event EventInteractive
  (bind _as_bp_lgamemode_first_person (Variables|Default|GetAs%20BP%20LGamemode%20First%20Person))
  (if (Variables|/Game/Luna/Blueprints/GameMode/Example_BP_LGamemodeFirstPerson.Example_BP_LGamemodeFirstPerson_C|GetSearchMode _as_bp_lgamemode_first_person)
    ;[1 1 1] Need to the Basement
    (if (Variables|/Game/Luna/Blueprints/GameMode/Example_BP_LGamemodeFirstPerson.Example_BP_LGamemodeFirstPerson_C|GetHasKey _as_bp_lgamemode_first_person)
      (CallFunction|LockOpens)
      (Audio|PlaySoundatLocation "/Game/Luna/Sounds/mixkit-creaky-door-open-195.mixkit-creaky-door-open-195" (Transformation|GetWorldLocation (Variables|Default|GetDoor_a)) "0, 0, 0" 1.0 1.0 0.0 0 0 0 0)
      (Utilities|FlowControl|FlipFlop
        (:A
          (bind _alpha (Timeline|Timeline Play)
            (:Update
              (Transformation|SetRelativeRotation (Variables|Default|GetDoor_a) (Math|Rotator|Lerp(Rotator) "0, 0, 0" "0.000000,-90.000000,0.000000" _alpha) false false))))
        (:B
          (Timeline|Timeline Reverse)))
      (else
        ;[1 1 1] Don't have the key
        (Utilities|FlowControl|DoOnce false :!label _label
          (:Completed
            (Audio|PlaySoundatLocation "/Game/Luna/Sounds/mixkit-gear-metallic-lock-sound-2858.mixkit-gear-metallic-lock-sound-2858" (Transformation|GetWorldLocation (Variables|Default|GetDoorBarricade_a)) "0, 0, 0" 1.0 1.0 0.0 0 0 0 0)
            (bind _returnvalue (UserInterface|CreateWidget "/Game/Luna/UI/Example_WPB_ItemTaking.Example_WPB_ItemTaking_C" (Game|GetPlayerController 0) (Variables|Default|GetItem%20Taking%20Desctiption)))
            (UserInterface|Viewport|AddtoViewport _returnvalue 0)
            (Utilities|FlowControl|Delay 3.0)
            (Widget|RemovefromParent _returnvalue)
            (goto _label Reset)))))
    (else
      ;[1 1 1] Don't go there
      (Utilities|FlowControl|DoOnce false :!label _label_2
        (:Completed
          (Audio|PlaySoundatLocation "/Game/Luna/Sounds/mixkit-gear-metallic-lock-sound-2858.mixkit-gear-metallic-lock-sound-2858" (Transformation|GetWorldLocation (Variables|Default|GetDoorBarricade_a)) "0, 0, 0" 1.0 1.0 0.0 0 0 0 0)
          (bind _returnvalue_2 (UserInterface|CreateWidget "/Game/Luna/UI/Example_WPB_LunaMonologue.Example_WPB_LunaMonologue_C" (Game|GetPlayerController 0) (Variables|Default|GetNoNeedToGoThere)))
          (UserInterface|Viewport|AddtoViewport _returnvalue_2 0)
          (Utilities|FlowControl|Delay 3.0)
          (Widget|RemovefromParent _returnvalue_2)
          (goto _label_2 Reset))))))

(fn ConstructionScript)