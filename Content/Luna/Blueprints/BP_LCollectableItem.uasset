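; Collectable pickup that counts down the items left when the Luna character touches it.
; A sphere collision overlap filters for BP_LunaCharacter, plays a 2D sound, then decrements ItemsLeft on Example_BP_LGamemodeFirstPerson.
; It then spawns a particle system at its location and destroys itself, both only if that game mode cast succeeds.
; The widget creation nodes are disconnected and never run.
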(event OnComponentBeginOverlap(SphereCollision)
  (params (OverlappedComponent :type Primitive%20Component%20Object%20Reference) (OtherActor :type Actor%20Object%20Reference) (OtherComp :type Primitive%20Component%20Object%20Reference) (OtherBodyIndex :type Integer) (bFromSweep :type Boolean) (SweepResult :type Hit%20Result%20Structure%20%28by%20ref%29))
  (Utilities|Casting|CastToBP_LunaCharacter OtherActor)
  (Audio|PlaySound2D 0 1.0 1.0 0.0 0 0)
  (bind _asbp_lgamemode_first_person (Utilities|Casting|CastToExample_BP_LGamemodeFirstPerson (Game|GetGameMode)))
  (bind _result (Math|Integer|DecrementInt (Variables|/Game/Luna/Blueprints/GameMode/Example_BP_LGamemodeFirstPerson.Example_BP_LGamemodeFirstPerson_C|GetItemsLeft _asbp_lgamemode_first_person))
    (:%20%20
      (Variables|/Game/Luna/Blueprints/GameMode/Example_BP_LGamemodeFirstPerson.Example_BP_LGamemodeFirstPerson_C|SetItemsLeft _asbp_lgamemode_first_person _result)
      (Niagara|SpawnSystematLocation 0 (Transformation|GetActorLocation))
      (Actor|DestroyActor))))

(event EventBeginPlay)

(event Collision|EventActorBeginOverlap
  (params (OtherActor :type Actor%20Object%20Reference)))

(event EventTick
  (params (DeltaSeconds :type Float%20%28single-precision%29)))

(fn ConstructionScript)