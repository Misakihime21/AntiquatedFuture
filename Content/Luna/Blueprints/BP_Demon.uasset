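; BP_Demon is a one-shot scripted demon sighting, built from eye and smoke components, that reacts as Luna approaches.
; Overlapping FeelingCollision briefly shows a "bad feeling" monologue widget.
; Overlapping EyesCollision plays a whoosh at an eye, destroys the eyes and smoke, briefly shows Luna's description of them, then destroys the actor.
; Both triggers filter for BP_LunaCharacter and use DoOnce.
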(event OnComponentBeginOverlap(FeelingCollision)
  (params (OverlappedComponent :type Primitive%20Component%20Object%20Reference) (OtherActor :type Actor%20Object%20Reference) (OtherComp :type Primitive%20Component%20Object%20Reference) (OtherBodyIndex :type Integer) (bFromSweep :type Boolean) (SweepResult :type Hit%20Result%20Structure%20%28by%20ref%29))
  (Utilities|Casting|CastToBP_LunaCharacter OtherActor)
  (Utilities|FlowControl|DoOnce false
    (:Completed
      (bind _returnvalue (UserInterface|CreateWidget "/Game/Luna/UI/Example_WPB_LunaMonologue.Example_WPB_LunaMonologue_C" (Game|GetPlayerController 0) (Variables|Default|GetBad%20feeling)))
      (UserInterface|Viewport|AddtoViewport _returnvalue 0)
      (Utilities|FlowControl|Delay 2.0)
      (Widget|RemovefromParent _returnvalue))))

(event OnComponentBeginOverlap(EyesCollision)
  (params (OverlappedComponent :type Primitive%20Component%20Object%20Reference) (OtherActor :type Actor%20Object%20Reference) (OtherComp :type Primitive%20Component%20Object%20Reference) (OtherBodyIndex :type Integer) (bFromSweep :type Boolean) (SweepResult :type Hit%20Result%20Structure%20%28by%20ref%29))
  (Utilities|Casting|CastToBP_LunaCharacter OtherActor)
  (Utilities|FlowControl|DoOnce false
    (:Completed
      (Audio|PlaySoundatLocation "/Game/Luna/Sounds/mixkit-quick-air-woosh-2605.mixkit-quick-air-woosh-2605" (Transformation|GetWorldLocation (Variables|Default|GetEye1)) "0, 0, 0" 1.0 1.0 0.0 0 0 0 0)
      (Components|DestroyComponent (Variables|Default|GetEye))
      (bind _returnvalue (UserInterface|CreateWidget "/Game/Luna/UI/Example_WPB_LunaMonologue.Example_WPB_LunaMonologue_C" (Game|GetPlayerController 0) (Variables|Default|GetEyesDescription)))
      (UserInterface|Viewport|AddtoViewport _returnvalue 0)
      (Utilities|FlowControl|Delay 2.0)
      (Widget|RemovefromParent _returnvalue)
      (Actor|DestroyActor))))

(event EventBeginPlay)

(event Collision|EventActorBeginOverlap
  (params (OtherActor :type Actor%20Object%20Reference)))

(event EventTick
  (params (DeltaSeconds :type Float%20%28single-precision%29)))

(fn ConstructionScript)