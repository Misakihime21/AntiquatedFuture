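; Trigger actor that plays Luna's closing dialogue with her mom and then loads the end screen level.
; When Luna enters the box while the game mode's EndingMode is set, a one-shot sequence disables input, turns her to Mom, starts a fade-out and calls the game mode's Ending.
; Timed delays then step through monologue and item-taking widgets, reused to show each character's lines, before opening L_EndScreen.
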(event OnComponentBeginOverlap(BoxCollision)
  (params (OverlappedComponent :type Primitive%20Component%20Object%20Reference) (OtherActor :type Actor%20Object%20Reference) (OtherComp :type Primitive%20Component%20Object%20Reference) (OtherBodyIndex :type Integer) (bFromSweep :type Boolean) (SweepResult :type Hit%20Result%20Structure%20%28by%20ref%29))
  (bind _asbp_luna_character (Utilities|Casting|CastToBP_LunaCharacter OtherActor))
  (if (Variables|/Game/Luna/Blueprints/GameMode/Example_BP_LGamemodeFirstPerson.Example_BP_LGamemodeFirstPerson_C|GetEndingMode (Variables|Default|GetAs%20BP%20LGamemode%20First%20Person))
    (Utilities|FlowControl|DoOnce false
      (:Completed
        (Input|DisableInput _asbp_luna_character (Game|GetPlayerController 0))
        (Default|RotationtoMom (Variables|Default|GetAs%20BP%20Luna%20Character))
        (bind _returnvalue (UserInterface|CreateWidget "/Game/Luna/UI/Example_WPB_LunaMonologue.Example_WPB_LunaMonologue_C" 0 (Variables|Default|GetLuna%20Says)))
        (UserInterface|Viewport|AddtoViewport _returnvalue 0)
        (bind _returnvalue_2 (UserInterface|CreateWidget "/Game/Luna/UI/Example_WBP_FadeScreen.Example_WBP_FadeScreen_C"))
        (UserInterface|Viewport|AddtoViewport _returnvalue_2 -1)
        (UserInterface|Animation|PlayAnimation _returnvalue_2 (Variables|/Game/Luna/UI/Example_WBP_FadeScreen.Example_WBP_FadeScreen_C|GetFadeOut _returnvalue_2) 0.0 1 "Forward" 0.5 false)
        (bind _asbp_lgamemode_first_person (Utilities|Casting|CastToExample_BP_LGamemodeFirstPerson (Game|GetGameMode)))
        (Default|Ending _asbp_lgamemode_first_person)
        (Utilities|FlowControl|Delay 4.0)
        (Widget|RemovefromParent _returnvalue)
        ;[1 0.3108 0.206] Oh, sweety
        (bind _returnvalue_3 (UserInterface|CreateWidget "/Game/Luna/UI/Example_WPB_ItemTaking.Example_WPB_ItemTaking_C" 0 (Variables|Default|GetMom%20Says)))
        (UserInterface|Viewport|AddtoViewport _returnvalue_3 0)
        (Utilities|FlowControl|Delay 3.0)
        (Widget|RemovefromParent _returnvalue_3)
        ;[1 0.2588 0.2339] Sorry for worrying you
        (bind _returnvalue_4 (UserInterface|CreateWidget "/Game/Luna/UI/Example_WPB_ItemTaking.Example_WPB_ItemTaking_C" 0 (Variables|Default|GetMom%20Says%202)))
        (UserInterface|Viewport|AddtoViewport _returnvalue_4 0)
        (Utilities|FlowControl|Delay 4.0)
        (Widget|RemovefromParent _returnvalue_4)
        ;[1 1 1] ...
        (bind _returnvalue_5 (UserInterface|CreateWidget "/Game/Luna/UI/Example_WPB_LunaMonologue.Example_WPB_LunaMonologue_C" 0 (Variables|Default|GetLuna%20Says%202)))
        (UserInterface|Viewport|AddtoViewport _returnvalue_5 0)
        (Utilities|FlowControl|Delay 1.5)
        ;[1 1 1] would you?
        (Widget|RemovefromParent _returnvalue_5)
        (bind _returnvalue_6 (UserInterface|CreateWidget "/Game/Luna/UI/Example_WPB_LunaMonologue.Example_WPB_LunaMonologue_C" 0 (Variables|Default|GetLuna%20Says%203)))
        (UserInterface|Viewport|AddtoViewport _returnvalue_6 0)
        (Utilities|FlowControl|Delay 4.0)
        (Widget|RemovefromParent _returnvalue_6)
        ;[1 0.2237 0.2187] Leave lights?
        (bind _returnvalue_7 (UserInterface|CreateWidget "/Game/Luna/UI/Example_WPB_ItemTaking.Example_WPB_ItemTaking_C" 0 (Variables|Default|GetMom%20Says%203)))
        (UserInterface|Viewport|AddtoViewport _returnvalue_7 0)
        (Utilities|FlowControl|Delay 4.0)
        (Widget|RemovefromParent _returnvalue_7)
        ;[1 1 1] I don't afraid
        (bind _returnvalue_8 (UserInterface|CreateWidget "/Game/Luna/UI/Example_WPB_LunaMonologue.Example_WPB_LunaMonologue_C" 0 (Variables|Default|GetLuna%20Says%204)))
        (UserInterface|Viewport|AddtoViewport _returnvalue_8 0)
        (Utilities|FlowControl|Delay 4.0)
        (Widget|RemovefromParent _returnvalue_8)
        (Game|OpenLevel(byName) "L_EndScreen")))))

(event EventBeginPlay
  (bind _asbp_lgamemode_first_person (Utilities|Casting|CastToExample_BP_LGamemodeFirstPerson (Game|GetGameMode)))
  (Variables|Default|SetAs%20BP%20LGamemode%20First%20Person _asbp_lgamemode_first_person)
  (bind _asbp_luna_character (Utilities|Casting|CastToBP_LunaCharacter (Game|GetPlayerCharacter 0)))
  (Variables|Default|SetAs%20BP%20Luna%20Character _asbp_luna_character)
  (bind _outactors (Actor|GetAllActorsOfClass 0))
  (Variables|Default|SetAs%20MomWaiting 0 0))

(fn ConstructionScript)