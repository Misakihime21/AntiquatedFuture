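; BP_PlateScreamer is a one-shot scare prop built around a plate that Luna can break.
; Luna overlapping the suspense collision plays a thunder sound at the plate, then destroys that trigger.
; The Interactive event plays a thunder impact, swaps the plate for its broken version, and briefly shows a Luna monologue widget.
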(event OnComponentBeginOverlap(CollisionSuspence)
  (params (OverlappedComponent :type Primitive%20Component%20Object%20Reference) (OtherActor :type Actor%20Object%20Reference) (OtherComp :type Primitive%20Component%20Object%20Reference) (OtherBodyIndex :type Integer) (bFromSweep :type Boolean) (SweepResult :type Hit%20Result%20Structure%20%28by%20ref%29))
  (Utilities|Casting|CastToBP_LunaCharacter OtherActor)
  (Utilities|FlowControl|DoOnce false
    (:Completed
      (Audio|PlaySoundatLocation "/Game/Luna/Sounds/mixkit-big-thunder-with-rain-1291.mixkit-big-thunder-with-rain-1291" (Transformation|GetWorldLocation (Variables|Default|GetPlate)) "0, 0, 0" 1.0 1.0 0.0 0 0 0 0)
      (Components|DestroyComponent (Variables|Default|GetCollisionSuspence)))))

(event EventInteractive
  (bind _plate (Variables|Default|GetPlate))
  (Utilities|FlowControl|DoOnce false
    (:Completed
      (Audio|PlaySoundatLocation "/Game/Luna/Sounds/mixkit-fast-thunder-impact-1279.mixkit-fast-thunder-impact-1279" (Transformation|GetWorldLocation _plate) "0, 0, 0" 1.0 1.0 0.5 0 0 0 0)
      (Components|DestroyComponent _plate)
      (Rendering|SetVisibility (Variables|Default|GetPlate_Broken) true false)
      (bind _returnvalue (UserInterface|CreateWidget "/Game/Luna/UI/Example_WPB_LunaMonologue.Example_WPB_LunaMonologue_C" (Game|GetPlayerController 0) (Variables|Default|GetLuna%20Says)))
      (UserInterface|Viewport|AddtoViewport _returnvalue 0)
      (Utilities|FlowControl|Delay 3.0)
      (Widget|RemovefromParent _returnvalue))))

(fn ConstructionScript)