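; BP_BasementKey is an interactive pickup for the basement key that records possession of it on the first-person game mode.
; BeginPlay caches the cast game mode reference.
; On Interactive it plays a key sound, sets HasKey, removes the key mesh and shows an item-taking widget with its description.
; After a short delay it removes the widget and destroys the actor.
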(event EventInteractive
  (Audio|PlaySoundatLocation "/Game/Luna/Sounds/mixkit-dropping-keys-in-the-floor-2839.mixkit-dropping-keys-in-the-floor-2839" (Transformation|GetWorldLocation (Variables|Default|GetKey_SM_Key)) "0, 0, 0" 1.0 1.0 0.0 0 0 0 0)
  (Variables|/Game/Luna/Blueprints/GameMode/Example_BP_LGamemodeFirstPerson.Example_BP_LGamemodeFirstPerson_C|SetHasKey (Variables|Default|GetAs%20BP%20LGamemode%20First%20Person) true)
  (bind _returnvalue (UserInterface|CreateWidget "/Game/Luna/UI/Example_WPB_ItemTaking.Example_WPB_ItemTaking_C" 0 (Variables|Default|GetItem%20Taking%20Desctiption)))
  (Components|DestroyComponent (Variables|Default|GetKey_SM_Key))
  (UserInterface|Viewport|AddtoViewport _returnvalue 0)
  (Utilities|FlowControl|Delay 3.0)
  (Widget|RemovefromParent _returnvalue)
  (Actor|DestroyActor))

(event EventBeginPlay
  (bind _asbp_lgamemode_first_person (Utilities|Casting|CastToExample_BP_LGamemodeFirstPerson (Game|GetGameMode)))
  (Variables|Default|SetAs%20BP%20LGamemode%20First%20Person _asbp_lgamemode_first_person))

(fn ConstructionScript)