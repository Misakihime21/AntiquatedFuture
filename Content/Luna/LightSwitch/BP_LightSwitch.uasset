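; Interactive wall light switch that toggles every BP_Light sharing its LightIndex, using lights gathered at BeginPlay.
; Each interaction plays a click and flips the switch mesh via a FlipFlop-driven timeline.
; In the game mode's SearchMode it leaves lights untouched, instead showing a one-time two-line Luna monologue and setting BasementCommentary.
; A resettable DoOnce gates interaction, blocking re-presses while the monologue plays.
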(event Custom|FlipFlop
  (Audio|PlaySoundatLocation "/Game/Luna/Sounds/mixkit-classic-click-1117.mixkit-classic-click-1117" (Transformation|GetWorldLocation (Variables|Default|Getlightswitch_CoverPlate_001)) "0, 0, 0" 1.0 1.0 0.0 0 0 0 0)
  (Utilities|FlowControl|FlipFlop
    (:A
      (bind _switchalpha (Timeline|Timeline_0 Play)
        (:Update
          (Transformation|SetRelativeRotation (Variables|Default|Getlightswitch_Switch_001) (Math|Rotator|MakeRotator 0.0 (Math|Float|Lerp 0.0 -1e+01 _switchalpha) 0.0) false false))))
    (:B
      (Timeline|Timeline_0 Reverse))))

(event EventBeginPlay
  (bind _asbp_lgamemode_first_person (Utilities|Casting|CastToExample_BP_LGamemodeFirstPerson (Game|GetGameMode)))
  (Variables|Default|SetAs%20BP%20LGamemode%20First%20Person _asbp_lgamemode_first_person)
  (bind _outactors (Actor|GetAllActorsOfClass "/Game/Luna/LightSwitch/BP_Light.BP_Light_C"))
  (for _array_element _outactors
    (Utilities|Array|Add (Variables|Lights|GetLightsArray) _array_element)))

(event EventInteractive
  (bind _as_bp_lgamemode_first_person (Variables|Default|GetAs%20BP%20LGamemode%20First%20Person))
  (Utilities|FlowControl|DoOnce false :!label _label
    (:Completed
      (CallFunction|FlipFlop)
      (if (Variables|/Game/Luna/Blueprints/GameMode/Example_BP_LGamemodeFirstPerson.Example_BP_LGamemodeFirstPerson_C|GetSearchMode (Variables|Default|GetAs%20BP%20LGamemode%20First%20Person))
        (if (Variables|/Game/Luna/Blueprints/GameMode/Example_BP_LGamemodeFirstPerson.Example_BP_LGamemodeFirstPerson_C|GetBasement%20Commentary _as_bp_lgamemode_first_person)
          (goto _label Reset)
          (else
            (Utilities|FlowControl|DoOnce false
              (:Completed
                (Variables|/Game/Luna/Blueprints/GameMode/Example_BP_LGamemodeFirstPerson.Example_BP_LGamemodeFirstPerson_C|SetBasement%20Commentary _as_bp_lgamemode_first_person true)
                (bind _returnvalue (UserInterface|CreateWidget "/Game/Luna/UI/Example_WPB_LunaMonologue.Example_WPB_LunaMonologue_C" (Game|GetPlayerController 0) (Variables|Default|GetLuna%20Says)))
                (UserInterface|Viewport|AddtoViewport _returnvalue 0)
                (Utilities|FlowControl|Delay 1.0)
                (Widget|RemovefromParent _returnvalue)
                (bind _returnvalue_2 (UserInterface|CreateWidget "/Game/Luna/UI/Example_WPB_LunaMonologue.Example_WPB_LunaMonologue_C" (Game|GetPlayerController 0) (Variables|Default|GetLuna%20Says_0)))
                (UserInterface|Viewport|AddtoViewport _returnvalue_2 0)
                (Utilities|FlowControl|Delay 3.0)
                (Widget|RemovefromParent _returnvalue_2)
                (goto _label Reset)))))
        (else
          (for _array_element (Variables|Lights|GetLightsArray)
            (if (== (Variables|/Game/Luna/LightSwitch/BP_Light.BP_Light_C|GetLight%20Index _array_element) (Variables|Lights|GetLight%20Index))
              (Class|BPILightsInterface|ToggleLights(Message) _array_element)
              (goto _label Reset)
              (else
                (goto _label Reset)))))))))

(fn ConstructionScript)