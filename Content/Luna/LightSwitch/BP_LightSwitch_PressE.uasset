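; BP_LightSwitch_PressE is a prompt actor for the light switch that shows or hides its Widget component, apparently a "Press E" hint.
; On BeginPlay it casts the player character to BP_LunaCharacter and caches the reference.
; Every Tick it polls that character's LookingAt flag, showing the widget while true and hiding it otherwise, without checking which object is being looked at.
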(event EventBeginPlay
  (|CallParentFunction)
  (bind _asbp_luna_character (Utilities|Casting|CastToBP_LunaCharacter (Game|GetPlayerCharacter 0)))
  (Variables|Default|SetAs%20BP%20Luna%20Character _asbp_luna_character))

(event EventTick
  (params (DeltaSeconds :type Float%20%28single-precision%29))
  (bind _widget (Variables|Default|GetWidget))
  (if (Variables|/Game/Luna/Blueprints/BP_LunaCharacter.BP_LunaCharacter_C|GetLookingAt (Variables|Default|GetAs%20BP%20Luna%20Character))
    (Development|SetHiddeninGame _widget false false)
    (else
      (Development|SetHiddeninGame _widget true false))))

(fn ConstructionScript
  (|CallParentFunction))