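; Big light switch actor that, on its first interaction only, enables the level's lights and advances the game state.
; BeginPlay caches every BP_Light, and Interactive sets each one's Works flag and plays a click sound.
; It then switches the first-person game mode from search to lighting mode and calls MomWaking.
; A brief Luna monologue widget appears, and a timeline tilts the switch mesh.
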(event Custom|LunaSays
  (bind _returnvalue (UserInterface|CreateWidget "/Game/Luna/UI/Example_WPB_LunaMonologue.Example_WPB_LunaMonologue_C" 0 (Variables|Default|GetLuna%20Says)))
  (UserInterface|Viewport|AddtoViewport _returnvalue 0)
  (Utilities|FlowControl|Delay 2.5)
  (Widget|RemovefromParent _returnvalue))

(event Custom|MakingLightsWork
  (for _array_element (Variables|Lights|GetLightsArray)
    (Variables|/Game/Luna/LightSwitch/BP_Light.BP_Light_C|SetWorks _array_element true)))

(event EventBeginPlay
  (bind _outactors (Actor|GetAllActorsOfClass "/Game/Luna/LightSwitch/BP_Light.BP_Light_C"))
  (for _array_element _outactors
    (Utilities|Array|Add (Variables|Lights|GetLightsArray) _array_element)))

(event EventInteractive
  (Utilities|FlowControl|DoOnce false
    (:Completed
      (CallFunction|MakingLightsWork)
      (Audio|PlaySoundatLocation "/Game/Luna/Sounds/mixkit-classic-click-1117.mixkit-classic-click-1117" (Transformation|GetWorldLocation (Variables|Default|Getlightswitch_CoverPlate_001)) "0, 0, 0" 1.0 1.0 0.0 0 0 0 0)
      (bind _asbp_lgamemode_first_person (Utilities|Casting|CastToExample_BP_LGamemodeFirstPerson (Game|GetGameMode)))
      (Variables|/Game/Luna/Blueprints/GameMode/Example_BP_LGamemodeFirstPerson.Example_BP_LGamemodeFirstPerson_C|SetLightingMode _asbp_lgamemode_first_person true)
      (Variables|/Game/Luna/Blueprints/GameMode/Example_BP_LGamemodeFirstPerson.Example_BP_LGamemodeFirstPerson_C|SetSearchMode _asbp_lgamemode_first_person false)
      (Default|MomWaking _asbp_lgamemode_first_person)
      (CallFunction|LunaSays)
      (bind _switchalpha (Timeline|Timeline Play)
        (:Update
          (Transformation|SetRelativeRotation (Variables|Default|Getlightswitch_Switch_001) (Math|Rotator|MakeRotator 0.0 (Math|Float|Lerp 0.0 -1e+01 _switchalpha) 0.0) false false))))))

(fn ConstructionScript)