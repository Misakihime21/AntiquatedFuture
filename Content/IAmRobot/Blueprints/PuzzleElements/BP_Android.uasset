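; BP_Android is a quest-giver NPC that asks the player for an amplifier module, then opens the path once it is received.
; Interacting checks the gamemode's item flag and shows dialogue through the player's speech system, with DoOnce and Delay throttling repeated lines.
; Completing the quest reveals the BP_Bridge actor, enables its collision and plays a sound.
; Tick toggles the widget from the player's LookingAt flag.
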(event Custom|PlatformAppears
  (bind _returnvalue (Actor|GetActorOfClass "/Game/IAmRobot/Blueprints/PuzzleElements/BP_Bridge.BP_Bridge_C"))
  (Rendering|SetVisibility (Variables|/Game/IAmRobot/Blueprints/PuzzleElements/BP_Bridge.BP_Bridge_C|GetBridge _returnvalue) true false)
  (Collision|SetCollisionEnabled (Variables|/Game/IAmRobot/Blueprints/PuzzleElements/BP_Bridge.BP_Bridge_C|GetBridge _returnvalue) "QueryAndPhysics")
  (Audio|PlaySoundatLocation "/Game/StarterContent/Audio/Collapse02.Collapse02" (Transformation|GetWorldLocation (Variables|/Game/IAmRobot/Blueprints/PuzzleElements/BP_Bridge.BP_Bridge_C|GetBridge _returnvalue)) "0, 0, 0" 1.0 1.0 0.0 0 0 0 0))

(event EventTick
  (params (DeltaSeconds :type Float%20%28single-precision%29))
  (bind _widget (Variables|Default|GetWidget))
  (if (Variables|/Game/IAmRobot/Blueprints/BP_RobotCharacter.BP_RobotCharacter_C|GetLooking%20At (Variables|Default|GetAs%20BP%20Robot%20Character))
    (Development|SetHiddeninGame _widget false false)
    (else
      (Development|SetHiddeninGame _widget true false))))

(event EventInteractive
  (bind _as_bp_robot_character (Variables|Default|GetAs%20BP%20Robot%20Character))
  (bind _as_bp_robot_character_2 (Variables|Default|GetAs%20BP%20Robot%20Character))
  (if (not (Variables|/Game/IAmRobot/Blueprints/GameMode/BP_GamemodeFirstPerson.BP_GamemodeFirstPerson_C|GetAndroidItemRecieved (Variables|Default|GetAs%20BP%20Gamemode%20First%20Person)))
    (Utilities|FlowControl|DoOnce false :!label _label
      (:Completed
        (Variables|/Game/IAmRobot/Blueprints/BP_RobotCharacter.BP_RobotCharacter_C|SetSpeechText _as_bp_robot_character_2 "Android: Locate the amplifier module, and I'll assist you further.")
        (Default|Speech _as_bp_robot_character_2)
        (Utilities|FlowControl|Delay 5.0)
        (goto _label Reset)))
    (elif (not (Variables|Default|GetQuestCompleted))
      (Variables|/Game/IAmRobot/Blueprints/BP_RobotCharacter.BP_RobotCharacter_C|SetSpeechText _as_bp_robot_character "Android: The emptiness in my ears is gone... The path for you is open.")
      (Default|Speech _as_bp_robot_character)
      (CallFunction|PlatformAppears)
      (Variables|Default|SetQuestCompleted true)
      (else
        (Utilities|FlowControl|DoOnce false :!label _label_2
          (:Completed
            (Variables|/Game/IAmRobot/Blueprints/BP_RobotCharacter.BP_RobotCharacter_C|SetSpeechText _as_bp_robot_character "Android: I can now hear the insects scuttling on my body.")
            (Default|Speech _as_bp_robot_character)
            (Utilities|FlowControl|Delay 5.0)
            (goto _label_2 Reset)))))))

(event EventBeginPlay
  (bind _asbp_robot_character (Utilities|Casting|CastToBP_RobotCharacter (Game|GetPlayerCharacter 0)))
  (Variables|Default|SetAs%20BP%20Robot%20Character _asbp_robot_character)
  (bind _asbp_gamemode_first_person (Utilities|Casting|CastToBP_GamemodeFirstPerson (Game|GetGameMode)))
  (Variables|Default|SetAs%20BP%20Gamemode%20First%20Person _asbp_gamemode_first_person))

(fn ConstructionScript)